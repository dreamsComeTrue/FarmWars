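; Animal character that the game can grab and drop, pausing its AI controller while held.
; On drop it launches upward and along the controller's forward vector, then restarts the AI.
; Capsule hits from anything but the player apply damage to itself and refresh the life widget from LifeLevel.
; On destruction it spawns a randomly tinted explosion effect and plays a crash sound.
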(event `self.OnAnimalGrabbed`
  (bind _asai_animal_controller (cast `/Game/AI/AI_AnimalController` (`AIBlueprintHelperLibrary.GetAIController` self)))
  (`/Game/AI/AI_AnimalController.StopAI` _asai_animal_controller))

(event `self.OnAnimalDropped`
  (bind _asai_animal_controller (cast `/Game/AI/AI_AnimalController` (`AIBlueprintHelperLibrary.GetAIController` self)))
  (bind (_returnvalue_x _returnvalue_y) (`KismetMathLibrary.BreakVector` (* (`self.GetActorForwardVector` _asai_animal_controller) 400.0)))
  (`CharacterMovementComponent.AddImpulse` (`self.CharacterMovement`) (`KismetMathLibrary.MakeVector` _returnvalue_x _returnvalue_y 700.0) true)
  (`/Game/AI/AI_AnimalController.RunAI` _asai_animal_controller))

(event `self.CapsuleComponent.OnComponentHit`
  (params (HitComponent :type "PrimitiveComponent Object Reference") (OtherActor :type "Actor Object Reference") (OtherComp :type "PrimitiveComponent Object Reference") (NormalImpulse :type "Vector Structure") (Hit :type "HitResult Structure (by ref)"))
  (cast `/Game/Blueprints/BP_PlayerCharacter` OtherActor
    (:`CastFailed`
      (`GameplayStatics.ApplyDamage` self 1.0)
      (`self.DamageTaken`))))

(event `DamageTaken`
  (bind _lifewidget (`self.LifeWidget`))
  (if (`KismetSystemLibrary.IsValid` _lifewidget)
    (bind _asui_life_widget (cast `/Game/UI/UI_LifeWidget` (`WidgetComponent.GetUserWidgetObject` _lifewidget)))
    (`/Game/UI/UI_LifeWidget.UpdateHealth` _asui_life_widget (`self.LifeLevel`))))

(event `self.ReceiveDestroyed`
  (bind _returnvalue (`NiagaraFunctionLibrary.SpawnSystemAtLocation` "/Game/FX/FX_Explode.FX_Explode" (`self.K2_GetActorLocation`)))
  (`FXSystemComponent.SetColorParameter` _returnvalue "User.ParticleColor" (`KismetMathLibrary.MakeColor` (`KismetMathLibrary.RandomFloat`) (`KismetMathLibrary.RandomFloat`) (`KismetMathLibrary.RandomFloat`)))
  (`GameplayStatics.PlaySound2D` "/Game/Sounds/SND_Crash_Cue.SND_Crash_Cue" 1.0 1.0 0.0 null null))

(fn `UserConstructionScript`)