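; Player character Blueprint that links the player to the on-screen UI and a movement animation.
; On BeginPlay it creates the UI_PlayerUI widget for the first player controller and adds it to the viewport.
; MoveAnimation plays a movement level sequence, or stops it and scrubs to a slightly negative time to reset it.
; InventoryItemChanged shows the widget's backpack element when the item is valid and hides it otherwise.
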(event `self.ReceiveBeginPlay`
  (bind _returnvalue (`|CreateWidget` "/Game/UI/UI_PlayerUI.UI_PlayerUI_C" (`GameplayStatics.GetPlayerController` 0)))
  (bind _output_get (set `self.UIWidget` _returnvalue))
  (`UserWidget.AddToViewport` _output_get 0))

(event `self.MoveAnimation`
  (params (shouldPlay :type Boolean))
  (bind _sequenceplayer (`ActorSequenceComponent.SequencePlayer` (`self.MovementSequence`)))
  (if shouldPlay
    (`MovieSceneSequencePlayer.Play` _sequenceplayer)
    (else
      (`MovieSceneSequencePlayer.Stop` _sequenceplayer)
      (`MovieSceneSequencePlayer.ScrubToSeconds` _sequenceplayer -0.2))))

(event `self.InventoryItemChanged`
  (params (InventoryItem :type "AnimalCharacter Object Reference"))
  (bind _backpack (`/Game/UI/UI_PlayerUI.Backpack` (`self.UIWidget`)))
  (`/Engine/EditorBlueprintResources/StandardMacros.IsValid` InventoryItem
    (:`Is Valid`
      (`Widget.SetVisibility` _backpack "Visible"))
    (:`Is Not Valid`
      (`Widget.SetVisibility` _backpack "Hidden"))))

(fn `UserConstructionScript`)